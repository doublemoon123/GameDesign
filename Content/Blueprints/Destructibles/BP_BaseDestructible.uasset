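; Base destructible actor that takes damage from first-person projectiles and awards score to the player.
; When a FirstPersonProjectile hits its Destructible component, it applies a large fixed point damage to the hit actor on every hit.
; A PointsAwarded flag ensures only the first such hit adds PointValue to the Score of player 0's FirstPersonCharacter.
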(event OnComponentHit(Destructible)
  (params (HitComponent :type Primitive%20Component%20Object%20Reference) (OtherActor :type Actor%20Object%20Reference) (OtherComp :type Primitive%20Component%20Object%20Reference) (NormalImpulse :type Vector :default "0, 0, 0") (Hit :type Hit%20Result%20Structure%20%28by%20ref%29))
  (bind (_bblockinghit _binitialoverlap _time _location _impactpoint _normal _impactnormal _physmat _hitactor) (Collision|BreakHitResult Hit))
  ;[1 1 1] Damage and add points
  (bind _asfirst_person_projectile (Utilities|Casting|CastToFirstPersonProjectile OtherActor))
  (Game|Damage|ApplyPointDamage _hitactor 5e+02 _impactpoint Hit 0 _asfirst_person_projectile "/Script/Engine.DamageType")
  (if (not (Variables|Default|GetPointsAwarded?))
    (Variables|Default|SetPointsAwarded? true)
    (bind _asfirst_person_character (Utilities|Casting|CastToFirstPersonCharacter (Game|GetPlayerCharacter 0)))
    (Variables|/Game/FirstPersonBP/Blueprints/FirstPersonCharacter.FirstPersonCharacter_C|SetScore _asfirst_person_character (+ (Variables|/Game/FirstPersonBP/Blueprints/FirstPersonCharacter.FirstPersonCharacter_C|GetScore _asfirst_person_character) (Variables|Default|GetPointValue)))))

(fn ConstructionScript)