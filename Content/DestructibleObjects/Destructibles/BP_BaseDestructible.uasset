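; Base destructible actor that tracks health and awards score to the player when it breaks.
; The construction script applies the configured mesh, and projectile hits deal heavy point damage.
; DamageObject, not called within this Blueprint, subtracts the damager's equipped weapon damage or a default unarmed amount, applying radius damage at zero health to shatter the mesh.
; Fracturing adds PointValue to the first player's character score, guarded to award once.
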(event OnComponentFracture(Destructible)
  (params (HitPoint :type Vector%20%28by%20ref%29 :default "0, 0, 0") (HitDirection :type Vector%20%28by%20ref%29 :default "0, 0, 0"))
  (bind _asfirst_person_character (Utilities|Casting|CastToFirstPersonCharacter (Game|Player|GetPlayerPawn 0)))
  (CallFunction|AssignPoints _asfirst_person_character))

(event OnComponentHit(Destructible)
  (params (HitComponent :type Primitive%20Component%20Object%20Reference) (OtherActor :type Actor%20Object%20Reference) (OtherComp :type Primitive%20Component%20Object%20Reference) (NormalImpulse :type Vector :default "0, 0, 0") (Hit :type Hit%20Result%20Structure%20%28by%20ref%29))
  (bind (_bblockinghit _binitialoverlap _time _location _impactpoint _normal _impactnormal _physmat _hitactor) (Collision|BreakHitResult Hit))
  (bind _asfirst_person_projectile (Utilities|Casting|CastToFirstPersonProjectile OtherActor))
  (Game|Damage|ApplyPointDamage _hitactor 1e+04 _impactpoint Hit 0 _asfirst_person_projectile "/Script/Engine.DamageType"))

(event EventBeginPlay)

(event Collision|EventActorBeginOverlap
  (params (OtherActor :type Actor%20Object%20Reference)))

(event EventTick
  (params (DeltaSeconds :type Float%20%28single-precision%29)))

(fn ConstructionScript
  (Class|DestructibleComponent|SetDestructibleMesh (Variables|Default|GetDestructible) (Variables|Default|GetMesh)))

(fn DamageObject
  (params (Hit :type Hit%20Result%20Structure) (Damager :type First%20Person%20Character%20Object%20Reference))
  (if (Variables|/Game/FirstPersonBP/Blueprints/FirstPersonCharacter.FirstPersonCharacter_C|GetHasItemEquipped Damager)
    (bind _asbp_base_weapon (Utilities|Casting|CastToBP_BaseWeapon (Variables|/Game/FirstPersonBP/Blueprints/FirstPersonCharacter.FirstPersonCharacter_C|GetEquippedItem Damager)))
    (LocalVariables|SetDamageToDeal (.Damage (Utilities|Struct|BreakFWeaponInfo (Variables|/Game/EquipableItems/Weapons/BP_BaseWeapon.BP_BaseWeapon_C|GetWeaponInfo _asbp_base_weapon))))
    (else
      (LocalVariables|SetDamageToDeal 5e+01)))
  (if (<= (- (Variables|Default|GetHealth) (LocalVariables|GetDamageToDeal)) 0.0)
    (Variables|Default|SetHealth 0.0)
    (Class|DestructibleComponent|ApplyRadiusDamage (Variables|Default|GetDestructible) (Math|Float|MakeLiteralFloat 1e+05) (.ImpactPoint (Collision|BreakHitResult Hit)) 2e+02 6.0 false)
    (else
      (Variables|Default|SetHealth (- (Variables|Default|GetHealth) (LocalVariables|GetDamageToDeal))))))

(fn AssignPoints
  (params (Character :type Actor%20Object%20Reference))
  (if (not (Variables|Default|GetPointsAwarded?))
    (Variables|Default|SetPointsAwarded? true)
    (bind _asfirst_person_character (Utilities|Casting|CastToFirstPersonCharacter Character))
    (Variables|/Game/FirstPersonBP/Blueprints/FirstPersonCharacter.FirstPersonCharacter_C|SetScore _asfirst_person_character (+ (Variables|/Game/FirstPersonBP/Blueprints/FirstPersonCharacter.FirstPersonCharacter_C|GetScore _asfirst_person_character) (Variables|Default|GetPointValue)))))