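; BP_BaseItem is the base actor for equipable items that an instigator picks up by interacting with it.
; The construction script stamps the item's own class into its ItemInfo struct, keeping the type and name.
; On Interaction, if the ItemClass passes a validity check, it sends ItemInfo to the instigator through a PickupItem message and destroys itself.
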(event EventInteraction
  (params (Instigator :type First%20Person%20Character%20Object%20Reference))
  (if (not (== (.itemclass (Variables|Default|GetItemInfo)) 0))
    (Class|BPIInteract|PickupItem(Message) Instigator (Variables|Default|GetItemInfo))
    (Actor|DestroyActor)))

(fn ConstructionScript
  (|CallParentFunction)
  (Variables|Default|SetItemInfo (Utilities|Struct|MakeFItemInfo (.itemtype (Variables|Default|GetItemInfo)) (.itemname (Variables|Default|GetItemInfo)) (Utilities|GetClass self))))