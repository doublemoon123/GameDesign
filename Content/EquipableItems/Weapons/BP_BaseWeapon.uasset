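; BP_BaseWeapon is the base melee weapon, handling the player's attack and the damage it deals.
; Attack plays a swing sound by attack type (lower-pitched for Heavy), then all types share one multi-sphere trace along the camera's forward vector out to the weapon's range.
; Each hit spawns WeaponInfo's VFX and sound, then damages BP_BaseDestructible or Robot_Worker actors.
; The trace uses the Camera channel and leaves debug drawing on.
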(event Custom|Attack
  (bind _weaponinfo (Variables|Default|GetWeaponInfo))
  (bind _weaponinfo_2 (Variables|Default|GetWeaponInfo))
  (bind _character_reference (Variables|Default|GetCharacter%20Reference))
  (bind _character_reference_2 (Variables|Default|GetCharacter%20Reference))
  (bind (_attackvfx _hitsfx) (Utilities|Struct|BreakFWeaponInfo _weaponinfo))
  (bind _returnvalue (Transformation|GetActorLocation _character_reference))
  (bind _firstpersoncamera (Variables|/Game/FirstPersonBP/Blueprints/FirstPersonCharacter.FirstPersonCharacter_C|GetFirstPersonCamera _character_reference))
  (bind _returnvalue_2 (Math|Vector|GetForwardVector _firstpersoncamera))
  (bind (_x _y _z) (Math|Vector|BreakVector _returnvalue))
  (bind _returnvalue_3 (* _returnvalue_2 (.range _weaponinfo_2)))
  (bind _returnvalue_4 (+ _returnvalue _returnvalue_3))
  (bind (_x_2 _y_2 _z_2) (Math|Vector|BreakVector _returnvalue_4))
  ;[1 1 1] Make attack and look if you hit anything, then call to apply damage to that object
  (switch Utilities|FlowControl|Switch|SwitchonEAttackType (.attacktype (Variables|Default|GetWeaponInfo))
    (:NewEnumerator1
      (Audio|SpawnSoundatLocation "/Game/SoundEffects/SledgeHammerSwingNew_Cue.SledgeHammerSwingNew_Cue" "0, 0, 0" "0, 0, 0" 1.0 1.2))
    (:NewEnumerator2
      (Audio|SpawnSoundatLocation "/Game/SoundEffects/SledgeHammerSwingNew_Cue.SledgeHammerSwingNew_Cue" "0, 0, 0" "0, 0, 0" 1.0 0.9))
    (:NewEnumerator3
      (Audio|SpawnSoundatLocation "/Game/SoundEffects/SledgeHammerSwingNew_Cue.SledgeHammerSwingNew_Cue" "0, 0, 0" "0, 0, 0" 1.0 0.7 0.1)))
  (bind (_outhits _returnvalue_5) (Collision|MultiSphereTraceByChannel (Math|Vector|MakeVector _x _y (+ _z 5e+01)) (Math|Vector|MakeVector _x_2 _y_2 (+ _z_2 4e+01)) 2e+01 "TraceTypeQuery2" false (Utilities|Array|MakeArray _character_reference) "ForDuration"))
  (if _returnvalue_5
    (for _array_element _outhits
      (Effects|SpawnEmitteratLocation _attackvfx (.Location (Collision|BreakHitResult _array_element)))
      (Audio|SpawnSoundatLocation _hitsfx (.Location (Collision|BreakHitResult _array_element)))
      (bind _asbp_base_destructible (Utilities|Casting|CastToBP_BaseDestructible (.HitActor (Collision|BreakHitResult _array_element)))
        (:then
          (Default|DamageObject _asbp_base_destructible _array_element _character_reference_2))
        (:CastFailed
          (bind _asrobot_worker (Utilities|Casting|CastToRobot_Worker (.HitActor (Collision|BreakHitResult _array_element))))
          (Default|TakeDamage _asrobot_worker _character_reference_2))))))

(event EventBeginPlay
  (bind _asfirst_person_character (Utilities|Casting|CastToFirstPersonCharacter (Game|GetPlayerCharacter 0)))
  (Variables|Default|SetCharacter%20Reference _asfirst_person_character))

(fn ConstructionScript
  (|CallParentFunction))