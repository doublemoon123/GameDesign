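; BP_BaseWeapon is a base weapon that performs the player's attack as a forward trace that deals damage.
; On BeginPlay it caches player 0's FirstPersonCharacter as the owner reference.
; Attack runs a debug-drawn multi sphere trace on the Camera channel from the character's location along its actor forward vector, as far as the WeaponInfo range.
; When the trace reports a hit, every returned actor receives WeaponInfo damage, with the character as damage causer.
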(event Custom|Attack
  (bind _character_reference (Variables|Default|GetCharacter%20Reference))
  (bind _returnvalue (Transformation|GetActorLocation _character_reference))
  (bind (_outhits _returnvalue_2) (Collision|MultiSphereTraceByChannel _returnvalue (+ _returnvalue (* (Transformation|GetActorForwardVector _character_reference) (.range (Variables|Default|GetWeaponInfo)))) 2e+01 "TraceTypeQuery2" false (Utilities|Array|MakeArray _character_reference) "ForDuration"))
  (if _returnvalue_2
    (for _array_element _outhits
      (Game|Damage|ApplyDamage (.HitActor (Collision|BreakHitResult _array_element)) (.Damage (Utilities|Struct|BreakFWeaponInfo (Variables|Default|GetWeaponInfo))) 0 (Variables|Default|GetCharacter%20Reference)))))

(event EventBeginPlay
  (bind _asfirst_person_character (Utilities|Casting|CastToFirstPersonCharacter (Game|GetPlayerCharacter 0)))
  (Variables|Default|SetCharacter%20Reference _asfirst_person_character))

(fn ConstructionScript
  (|CallParentFunction))